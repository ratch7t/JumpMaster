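; BP_Player is a 2D side-scrolling player character with a Paper2D flipbook sprite.
; Input moves it along the world X axis and triggers jumping.
; Each tick it picks the fall, run or idle flipbook from movement state and velocity.
; It also turns the controller yaw to face the direction of X velocity, flipping the character left or right.
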(event `InputAction|Jump`
  (params (Key :type "Key Structure"))
  ;[1 1 1] Jump Movement
  (:`Pressed`
    (`self.Jump`))
  (:`Released`
    (`self.StopJumping`)))

(event `self.ReceiveTick`
  (params (DeltaSeconds :type "Float (single-precision)"))
  (bind _returnvalue (`GameplayStatics.GetPlayerController` 0))
  (bind _returnvalue_x (`KismetMathLibrary.BreakVector` (`self.GetVelocity`)))
  (`|ExecutionSequence`
    (:`then_0`
      (if (`NavMovementComponent.IsFalling` (`self.CharacterMovement`))
        (`PaperFlipbookComponent.SetFlipbook` (`self.Sprite`) (`self.FB_Fall`))
        (elif (!= (`KismetMathLibrary.VSize` (`self.GetVelocity`)) 0.0)
          (`PaperFlipbookComponent.SetFlipbook` (`self.Sprite`) (`self.FB_Run `))
          (else
            (`PaperFlipbookComponent.SetFlipbook` (`self.Sprite`) (`self.FB_Idle`))))))
    (:`then_1`
      (`/Engine/EditorBlueprintResources/StandardMacros.CompareFloat` _returnvalue_x
        (:`>`
          (`Controller.SetControlRotation` _returnvalue (`KismetMathLibrary.MakeRotator` 0.0)))
        (:`<`
          (`Controller.SetControlRotation` _returnvalue (`KismetMathLibrary.MakeRotator` 0.0 0.0 180.0)))))))

(event `InputAxis|Move`
  (params (AxisValue :type "Float (single-precision)"))
  ;[1 1 1] Movement of the player
  (`self.AddMovementInput` (1.0 0.0 0.0) AxisValue))

(fn `UserConstructionScript`)